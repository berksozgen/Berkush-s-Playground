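; Player character Blueprint that applies saved, per-part color customization and shares it across the network.
; On BeginPlay, the locally controlled character loads BSG_EpicCustomization and, on success, sends the data through a server event that stores and multicasts it.
; It then reapplies stored data on every existing BP_StrikeCharacter to cover players who were ready earlier.
; SetupCustomization, also run at construction, creates dynamic material instances per mesh slot and sets their Color scalar.
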(event `SetupPreReadyCharacters`
  (bind _outactors (`GameplayStatics.GetAllActorsOfClass` "BP_StrikeCharacter_C"))
  (for _array_element _outactors
    (`self.SetupCustomization` _array_element (`/Game/Blueprints/Character/BP_StrikeCharacter.CustomizationData` _array_element))))

(event `Server_SetCustomizationData`
  (params (CustomizationData :type "/BerkushOnline/Customization/EpicCharacter/F_EpicCharacterCustomization Structure"))
  (bind _output_get (set `self.CustomizationData` CustomizationData))
  (`self.Multicast_SetCustomizationData` _output_get))

(event `Multicast_SetCustomizationData`
  (params (CustomizationData :type "/BerkushOnline/Customization/EpicCharacter/F_EpicCharacterCustomization Structure"))
  (`self.SetupCustomization` CustomizationData))

(event `self.ReceiveBeginPlay`
  (`parent.ReceiveBeginPlay`)
  (if (`self.IsLocallyControlled`)
    (bind _returnvalue (`GameplayStatics.CreateSaveGameObject` "/BerkushOnline/Customization/EpicCharacter/BSG_EpicCustomization.BSG_EpicCustomization_C"))
    (bind (_issucsess _data) (`/BerkushOnline/Customization/EpicCharacter/BSG_EpicCustomization.LoadCustomization` _returnvalue))
    (if _issucsess
      (`self.Server_SetCustomizationData` _data)
      (`self.SetupPreReadyCharacters`))))

(fn `SetupCustomization`
  (params (Data :type "/BerkushOnline/Customization/EpicCharacter/F_EpicCharacterCustomization Structure"))
  (bind (_tunic _hood _bedroll _backpack _boots _sleevesshorts _skin _head) (break `/BerkushOnline/Customization/EpicCharacter/F_EpicCharacterCustomization` Data))
  (bind _mesh (`self.Mesh`))
  (bind _returnvalue (`PrimitiveComponent.CreateDynamicMaterialInstance` _mesh 0 "/BerkushOnline/Customization/EpicCharacter/Materials/MI_EpicCharacter_Tunic.MI_EpicCharacter_Tunic" "None"))
  (`MaterialInstanceDynamic.SetScalarParameterValue` _returnvalue "Color" _tunic)
  (bind _returnvalue_2 (`PrimitiveComponent.CreateDynamicMaterialInstance` _mesh 1 "/BerkushOnline/Customization/EpicCharacter/Materials/MI_EpicCharacter_Hood.MI_EpicCharacter_Hood" "None"))
  (`MaterialInstanceDynamic.SetScalarParameterValue` _returnvalue_2 "Color" _hood)
  (bind _returnvalue_3 (`PrimitiveComponent.CreateDynamicMaterialInstance` _mesh 2 "/BerkushOnline/Customization/EpicCharacter/Materials/MI_EpicCharacter_Bedroll.MI_EpicCharacter_Bedroll" "None"))
  (`MaterialInstanceDynamic.SetScalarParameterValue` _returnvalue_3 "Color" _bedroll)
  (bind _returnvalue_4 (`PrimitiveComponent.CreateDynamicMaterialInstance` _mesh 3 "/BerkushOnline/Customization/EpicCharacter/Materials/MI_EpicCharacter_Backpack.MI_EpicCharacter_Backpack" "None"))
  (`MaterialInstanceDynamic.SetScalarParameterValue` _returnvalue_4 "Color" _backpack)
  (bind _returnvalue_5 (`PrimitiveComponent.CreateDynamicMaterialInstance` _mesh 4 "/BerkushOnline/Customization/EpicCharacter/Materials/MI_EpicCharacter_Boots.MI_EpicCharacter_Boots" "None"))
  (`MaterialInstanceDynamic.SetScalarParameterValue` _returnvalue_5 "Color" _boots)
  (bind _returnvalue_6 (`PrimitiveComponent.CreateDynamicMaterialInstance` _mesh 5 "/BerkushOnline/Customization/EpicCharacter/Materials/MI_EpicCharacter_SleevesShorts.MI_EpicCharacter_SleevesShorts" "None"))
  (`MaterialInstanceDynamic.SetScalarParameterValue` _returnvalue_6 "Color" _sleevesshorts)
  (bind _returnvalue_7 (`PrimitiveComponent.CreateDynamicMaterialInstance` _mesh 6 "/BerkushOnline/Customization/EpicCharacter/Materials/MI_EpicCharacter_Skin.MI_EpicCharacter_Skin" "None"))
  (`MaterialInstanceDynamic.SetScalarParameterValue` _returnvalue_7 "Color" _skin)
  (bind _returnvalue_8 (`PrimitiveComponent.CreateDynamicMaterialInstance` _mesh 7 "/BerkushOnline/Customization/EpicCharacter/Materials/MI_EpicCharacter_Head.MI_EpicCharacter_Head" "None"))
  (`MaterialInstanceDynamic.SetScalarParameterValue` _returnvalue_8 "Color" _head))

(fn `UserConstructionScript`
  (`parent.UserConstructionScript`)
  (`self.SetupCustomization` (`self.CustomizationData`)))