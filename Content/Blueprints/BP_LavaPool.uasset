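; BP_LavaPool is a lava hazard that damages any StrikeCharacter at or below its height.
; On the server, a BeginPlay loop refreshes a cached list of characters every five seconds.
; Tick applies frame-rate-scaled damage to each valid character, using only a Z comparison with no overlap or horizontal bounds check.
; The victim is its own damage causer, and its instigator controller receives credit.
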(event `self.ReceiveBeginPlay`
  (`/Engine/EditorBlueprintResources/ActorMacros.Switch Has Authority`
    (:`Authority`
      (bind _outactors (`GameplayStatics.GetAllActorsOfClass` "/Script/BerkushsPlayground.StrikeCharacter" :!label _label))
      (set `self.PlayerArray` _outactors)
      (`KismetSystemLibrary.Delay` 5.0)
      (goto _label))))

(event `self.ReceiveTick`
  (params (DeltaSeconds :type "Float (single-precision)"))
  (bind (_returnvalue_x _returnvalue_y _returnvalue_z) (`KismetMathLibrary.BreakVector` (`self.K2_GetActorLocation`)))
  (`/Engine/EditorBlueprintResources/ActorMacros.Switch Has Authority`
    (:`Authority`
      (for _array_element (`self.PlayerArray`)
        (`/Engine/EditorBlueprintResources/StandardMacros.IsValid` _array_element
          (:`Is Valid`
            (bind (_returnvalue_x_2 _returnvalue_y_2 _returnvalue_z_2) (`KismetMathLibrary.BreakVector` (`self.K2_GetActorLocation` _array_element)))
            (if (<= _returnvalue_z_2 _returnvalue_z)
              (`GameplayStatics.ApplyDamage` _array_element (* DeltaSeconds (`self.DamagePerSecond`)) (`self.GetInstigatorController` _array_element) _array_element "/Script/Engine.DamageType"))))))))

(fn `UserConstructionScript`)