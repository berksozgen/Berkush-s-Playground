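; TestActor is a test actor that cycles the look of its Polygon skeletal mesh over time.
; The construction script creates a dynamic material instance from the mesh's first material and assigns it back to that slot.
; Tick ramps a hue value that drives the material's hue shift parameter.
; Each time the value passes one, it resets and swaps in a random texture and skeletal mesh from arrays.
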(event `self.ReceiveTick`
  (params (DeltaSeconds :type "Float (single-precision)"))
  (bind _dynamicinst (`self.DynamicInst`))
  (bind _currenthuevalue (`self.CurrentHueValue`))
  (if (<= _currenthuevalue 1.0)
    (set `self.CurrentHueValue` (+ _currenthuevalue (/ DeltaSeconds 1.0)))
    (else
      (set `self.CurrentHueValue` 0.0)
      (`MaterialInstanceDynamic.SetTextureParameterValue` _dynamicinst "Texture" (`KismetArrayLibrary.Array_Random` (`self.TextureArray`)))
      (`SkeletalMeshComponent.SetSkeletalMeshAsset` (`self.Polygon`) (`KismetArrayLibrary.Array_Random` (`self.SkeletonsArray`)))))
  (`MaterialInstanceDynamic.SetScalarParameterValue` _dynamicinst "HueShiftAll" _currenthuevalue))

(fn `UserConstructionScript`
  (bind _polygon (`self.Polygon`))
  (bind _returnvalue (`PrimitiveComponent.CreateDynamicMaterialInstance` _polygon 0 (`PrimitiveComponent.GetMaterial` (`self.Polygon`) 0) "None"))
  (bind _output_get (set `self.DynamicInst` _returnvalue))
  (`PrimitiveComponent.SetMaterial` _polygon 0 _output_get))