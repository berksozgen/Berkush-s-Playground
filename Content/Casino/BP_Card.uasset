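; BP_Card is a casino playing card actor with front and back sprites taken from the DT_WhiteCardSprites data table.
; The construction script sets the back sprite from the "Back" row.
; On BeginPlay, SetFrontFace builds a row name from the Turkish suit name and CardPower to set the front sprite.
; All three ShowFrontFace cases run that same lookup, so the value does not change the result.
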(event `self.ReceiveBeginPlay`
  (`parent.ReceiveBeginPlay`)
  (`self.SetFrontFace`))

(fn `SetFrontFace`
  (switch `int` (`self.ShowFrontFace`)
    (:`0`
      _)
    (:`1`
      _)
    (:`2`
      _))
  (bind _returnvalue (`|GetDataTableRow` "/Game/Casino/DT_WhiteCardSprites.DT_WhiteCardSprites" (`KismetStringLibrary.Conv_StringToName` (`KismetTextLibrary.Conv_TextToString` (`|FormatText` "{CardSymbol}_{CardPower}" (select `byte` (`self.CardSymbol`) :`0` "Sinek" :`1` "Maca" :`2` "Karo" :`3` "Kupa" :!type "Name") (`self.CardPower`)))))
    (:`then`
      (`PaperSpriteComponent.SetSprite` (`self.CardFront`) (`.Sprite` (break `CardSprites` _returnvalue))))))

(fn `UserConstructionScript`
  (bind _returnvalue (`|GetDataTableRow` "/Game/Casino/DT_WhiteCardSprites.DT_WhiteCardSprites" "Back")
    (:`then`
      (`PaperSpriteComponent.SetSprite` (`self.CardBack`) (`.Sprite` (break `CardSprites` _returnvalue))))))