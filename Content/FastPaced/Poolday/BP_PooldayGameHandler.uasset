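; Game handler for the Poolday mode that spawns player characters for their selected team.
; SpawnPlayer routes through a server event to a multicast, which spawns a BP_BerkushsLALSCharacter and has the selecting controller possess it, so spawn and possession run inside the multicast.
; Spawn transforms come from random points within the Red or Blue spawn area bounds, while Spectator uses the handler's own transform.
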(event `Server_SpawnPlayer`
  (params (Input :type "/Game/FastPaced/Poolday/FS_StrikeTeamSelector Structure"))
  (`KismetSystemLibrary.PrintString` "Hello")
  (`self.MulticastSpawnPlayer` Input))

(event `MulticastSpawnPlayer`
  (params (Input :type "/Game/FastPaced/Poolday/FS_StrikeTeamSelector Structure"))
  (bind _returnvalue (`|SpawnActorFromClass` "/Game/Blueprints/BP_BerkushsLALSCharacter.BP_BerkushsLALSCharacter_C" (`self.GetSpawnTransformInArea` Input) "AlwaysSpawn" "MultiplyWithRoot" null null))
  (`Controller.Possess` (`.WhoSelected_5_34786D77A741F756BE3406968E1B4CA3` (break `/Game/FastPaced/Poolday/FS_StrikeTeamSelector` Input)) _returnvalue))

(event `SpawnPlayer`
  (params (Input :type "/Game/FastPaced/Poolday/FS_StrikeTeamSelector Structure"))
  (`self.Server_SpawnPlayer` Input))

(fn `GetSpawnTransformInArea`
  (params (Input :type "/Game/FastPaced/Poolday/FS_StrikeTeamSelector Structure"))
  (returns (Transform :type "Transform Structure"))
  (bind (_origin _boxextent) (`KismetSystemLibrary.GetComponentBounds` (`self.BlueTeamSpawnArea`)))
  (bind (_origin_2 _boxextent_2) (`KismetSystemLibrary.GetComponentBounds` (`self.RedTeamSpawnArea`)))
  (return (select `EBerkushStrikePlayerTeam` (`.SelectedTeam_2_2EFE574F764FBDC863FC638F7DB9FD55` (break `/Game/FastPaced/Poolday/FS_StrikeTeamSelector` Input)) :`Red` (`KismetMathLibrary.MakeTransform` (`KismetMathLibrary.RandomPointInBoundingBox` _origin_2 _boxextent_2)) :`Blue` (`KismetMathLibrary.MakeTransform` (`KismetMathLibrary.RandomPointInBoundingBox` _origin _boxextent)) :`Spectator` (`self.GetTransform`))))

(fn `UserConstructionScript`)