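; BP_PooldayGameMode is the game mode for the Poolday map, controlling where player pawns spawn.
; Its construction script caches the level's BerkushStrikeGameHandler.
; The SpawnDefaultPawnAtTransform override spawns and possesses a BP_BerkushsLALSCharacter at a random point in the handler's red team spawn area, for every player.
; Spawns ignore collision and face from the area's center toward the handler, keeping only the incoming transform's scale.
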(event `self.ReceiveBeginPlay`)

(fn `SpawnDefaultPawnAtTransform`
  (params (NewPlayer :type "Controller Object Reference") (SpawnTransform :type "Transform Structure (by ref)"))
  (returns (ReturnValue :type "Pawn Object Reference"))
  (bind _gamehandler (`self.GameHandler`))
  (bind (_origin _boxextent) (`KismetSystemLibrary.GetComponentBounds` (`BerkushStrikeGameHandler.RedTeamSpawnArea` _gamehandler)))
  (bind _returnvalue (`|SpawnActorFromClass` "/Game/Blueprints/BP_BerkushsLALSCharacter.BP_BerkushsLALSCharacter_C" (`KismetMathLibrary.MakeTransform` (`KismetMathLibrary.RandomPointInBoundingBox` _origin _boxextent) (`KismetMathLibrary.FindLookAtRotation` _origin (`self.K2_GetActorLocation` _gamehandler)) (.scale SpawnTransform)) "AlwaysSpawn" "MultiplyWithRoot" null null))
  (`Controller.Possess` NewPlayer _returnvalue)
  (return _returnvalue))

(fn `UserConstructionScript`
  (bind _returnvalue (`GameplayStatics.GetActorOfClass` "/Script/BerkushStrike.BerkushStrikeGameHandler"))
  (set `self.GameHandler` _returnvalue))